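; Player Blueprint that handles HUD, audio and weapon visual feedback, plus pause and reload input.
; Health, ammo, weapon icon and reload events update the MainHUD held by BP_GameMode, with sounds on hit and heal.
; Weapon changes swap the Gun mesh with a pickup sound, scaling the grenade launcher down.
; Health values and reload logic are not defined here; pausing opens WBP_Pause with UI-only input and a cursor.
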(event Input|EnhancedActionEvents|EnhancedInputActionIA_Pause
  (params (ActionValue :type Boolean) (ElapsedSeconds :type Float%20%28double-precision%29) (TriggeredSeconds :type Float%20%28double-precision%29) (InputAction :type Input%20Action%20Object%20Reference :default "/Game/Input/Actions/IA_Pause.IA_Pause"))
  (bind _returnvalue (Game|GetPlayerController 0))
  (bind _returnvalue_2 (UserInterface|CreateWidget "/Game/Blueprints/WBP_Pause.WBP_Pause_C"))
  (UserInterface|Viewport|AddtoViewport _returnvalue_2 0)
  (Game|SetGamePaused true)
  (Input|SetInputModeUIOnly _returnvalue 0 "DoNotLock" false)
  (Variables|/Script/Engine.PlayerController|SetbShowMouseCursor _returnvalue true))

(event Input|EnhancedActionEvents|EnhancedInputActionIA_Reload
  (params (ActionValue :type Boolean) (ElapsedSeconds :type Float%20%28double-precision%29) (TriggeredSeconds :type Float%20%28double-precision%29) (InputAction :type Input%20Action%20Object%20Reference :default "/Game/Input/Actions/IA_Reload.IA_Reload"))
  (Class|SSCharacter|Reload))

(event EventBeginPlay
  (bind _asbp_game_mode (Utilities|Casting|CastToBP_GameMode (Game|GetGameMode)))
  (Variables|Default|SetMyHUD (Variables|/Game/Blueprints/BP_GameMode.BP_GameMode_C|GetMainHUD _asbp_game_mode))
  (Variables|/Script/Engine.PlayerController|SetbShowMouseCursor (Game|GetPlayerController 0) false))

(event Collision|EventActorBeginOverlap
  (params (OtherActor :type Actor%20Object%20Reference)))

(event EventTick
  (params (DeltaSeconds :type Float%20%28single-precision%29)))

(event EventOnHitVisuals
  (bind _asbp_game_mode (Utilities|Casting|CastToBP_GameMode (Game|GetGameMode)))
  (Class|SSHUDWidget|UpdateHealth (Variables|/Game/Blueprints/BP_GameMode.BP_GameMode_C|GetMainHUD _asbp_game_mode) (Variables|Default|GetCurrentHealth) (Variables|Default|GetMaxHealth))
  (Default|PlayHitAnim (Variables|/Game/Blueprints/BP_GameMode.BP_GameMode_C|GetMainHUD _asbp_game_mode))
  (Audio|PlaySound2D "/Game/Sounds/Effects/MS_RobotDamage.MS_RobotDamage" 1.0 1.0 0.0 0 0))

(event EventOnUpdateWeaponMesh
  (params (NewMesh :type Static%20Mesh%20Object%20Reference))
  (bind _gun (Variables|Default|GetGun))
  (if (== NewMesh "/Game/Data/SSWeapons/SM_GrenadeLauncher.SM_GrenadeLauncher")
    (Components|StaticMesh|SetStaticMesh _gun NewMesh)
    (Transformation|SetWorldScale3D _gun "0.800000,0.800000,0.800000")
    (else
      (Components|StaticMesh|SetStaticMesh _gun NewMesh)
      (Transformation|SetWorldScale3D _gun "1.000000,1.000000,1.000000")))
  (Audio|PlaySound2D "/Game/Sounds/Weapons/PickupWeapon.PickupWeapon" 3.0 1.0 0.0 0 0))

(event EventOnUpdateAmmoUI
  (params (AmmoCount :type Integer) (MaxAmmoCount :type Integer))
  (bind _asbp_game_mode (Utilities|Casting|CastToBP_GameMode (Game|GetGameMode)))
  (Default|UpdateAmmo (Variables|/Game/Blueprints/BP_GameMode.BP_GameMode_C|GetMainHUD _asbp_game_mode) AmmoCount MaxAmmoCount))

(event EventOnHealVisuals
  (bind _asbp_game_mode (Utilities|Casting|CastToBP_GameMode (Game|GetGameMode)))
  (Class|SSHUDWidget|UpdateHealth (Variables|/Game/Blueprints/BP_GameMode.BP_GameMode_C|GetMainHUD _asbp_game_mode) (Variables|Default|GetCurrentHealth) (Variables|Default|GetMaxHealth))
  (Default|PlayHealAnim (Variables|/Game/Blueprints/BP_GameMode.BP_GameMode_C|GetMainHUD _asbp_game_mode))
  (Audio|PlaySound2D "/Game/Sounds/Effects/MS_RobotHeal.MS_RobotHeal" 1.0 1.0 0.0 0 0))

(event EventOnReloadStart
  (params (Duration :type Float%20%28single-precision%29))
  (Default|StartReloadUI (Variables|Default|GetMyHUD) Duration))

(event EventOnUpdateWeaponIcon
  (params (NewIcon :type Texture%202D%20Object%20Reference))
  (bind _asbp_game_mode (Utilities|Casting|CastToBP_GameMode (Game|GetGameMode)))
  (Default|UpdateIcon (Variables|/Game/Blueprints/BP_GameMode.BP_GameMode_C|GetMainHUD _asbp_game_mode) NewIcon))

(fn ConstructionScript)