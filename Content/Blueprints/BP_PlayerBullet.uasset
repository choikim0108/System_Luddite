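; Player bullet Blueprint that handles impact feedback and decides when the projectile is destroyed.
; Overlapping an SSDamageInterface actor spawns blood and a random-pitch hit sound, while a blocking hit spawns asphalt debris and a wall sound along the surface normal.
; Both paths trigger HUD hit feedback through BP_GameMode, then destroy the bullet unless pierces or ricochets respectively remain.
; Damage and count updates are not handled in this graph.
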(event EventBeginPlay)

(event EventTick
  (params (DeltaSeconds :type Float%20%28single-precision%29)))

(event Collision|EventHit
  (params (MyComp :type Primitive%20Component%20Object%20Reference) (Other :type Actor%20Object%20Reference) (OtherComp :type Primitive%20Component%20Object%20Reference) (bSelfMoved :type Boolean) (HitLocation :type Vector :default "0, 0, 0") (HitNormal :type Vector :default "0, 0, 0") (NormalImpulse :type Vector :default "0, 0, 0") (Hit :type Hit%20Result%20Structure%20%28by%20ref%29))
  (bind _returnvalue (Math|Rotator|MakeRotfromX HitNormal))
  (Effects|SpawnEmitteratLocation "/Game/Realistic_Starter_VFX_Pack_Vol2/Particles/Hit/P_Asphalt.P_Asphalt" HitLocation _returnvalue)
  (Audio|SpawnSoundatLocation "/Game/Sounds/Effects/MS_BulletHitWall.MS_BulletHitWall" HitLocation _returnvalue 0.5 (Math|Random|RandomFloatinRange 0.1 1.5) 0.0 0 0)
  (bind _asbp_game_mode (Utilities|Casting|CastToBP_GameMode (Game|GetGameMode)))
  (Default|ShowHitFeedback (Variables|/Game/Blueprints/BP_GameMode.BP_GameMode_C|GetMainHUD _asbp_game_mode))
  (if (not (> (Variables|Default|GetCurrentRicochetCount) 0))
    (Actor|DestroyActor)))

(event Collision|EventActorBeginOverlap
  (params (OtherActor :type Actor%20Object%20Reference))
  (bind _returnvalue (Transformation|GetActorLocation))
  (bind _returnvalue_2 (Transformation|GetActorRotation))
  (if (Utilities|DoesObjectImplementInterface OtherActor "/Script/SuperSimple.SSDamageInterface")
    (Effects|SpawnEmitteratLocation "/Game/Realistic_Starter_VFX_Pack_Vol2/Particles/Blood/P_Blood_Splat_Cone.P_Blood_Splat_Cone" _returnvalue _returnvalue_2 "2.000000,2.000000,2.000000")
    (Audio|SpawnSoundatLocation "/Game/Sounds/Effects/MS_BulletHitEnemy.MS_BulletHitEnemy" _returnvalue _returnvalue_2 1.0 (Math|Random|RandomFloatinRange 0.1 1.5) 0.0 0 0)
    (bind _asbp_game_mode (Utilities|Casting|CastToBP_GameMode (Game|GetGameMode)))
    (Default|ShowHitFeedback (Variables|/Game/Blueprints/BP_GameMode.BP_GameMode_C|GetMainHUD _asbp_game_mode))
    (if (not (> (Variables|Default|GetCurrentPierceCount) 0))
      (Actor|DestroyActor))))

(fn ConstructionScript)