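; Game mode that runs the HUD, music, level-up upgrades and game-over screen.
; BeginPlay creates the HUD, starts a random music track and forwards score changes to the HUD.
; Level-up pauses play and offers three shuffled augments, then applies the pick to player stats, projectiles or weapon and resumes.
; Tick eases music pitch down when player health is at one or below, while game over pauses and shows score and wave.
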(event Custom|OnScoreChanged_Event
  (params (CurrentScore :type Integer) (CurrentLevel :type Integer))
  (Class|SSHUDWidget|UpdateScore (Variables|Default|GetMainHUD) CurrentScore))

(event Custom|LevelUpSequence
  (bind _returnvalue (Game|GetPlayerController 0))
  (bind _allaugments (Variables|Default|GetAllAugments))
  (Game|SetGamePaused true)
  (Input|SetInputModeUIOnly _returnvalue 0 "DoNotLock" false)
  (Variables|/Script/Engine.PlayerController|SetbShowMouseCursor _returnvalue true)
  (Utilities|Array|Shuffle _allaugments)
  (bind _returnvalue_2 (UserInterface|CreateWidget "/Game/Blueprints/WBP_Upgrade.WBP_Upgrade_C" _returnvalue))
  (bind _output_get (Variables|Default|SetActiveUpgradeWidget _returnvalue_2))
  (Class|SSUpgradeWidget|SetupOptions _output_get (Utilities|Array|MakeArray (Utilities|Array|Get(acopy) _allaugments) (Utilities|Array|Get(acopy) _allaugments 1) (Utilities|Array|Get(acopy) _allaugments 2)))
  (UserInterface|Viewport|AddtoViewport _output_get 0)
  (EventDispatchers|AssignOnAugmentSelected _output_get (delegate Custom|OnAugmentSelected_Event)))

(event Custom|OnAugmentSelected_Event
  (params (SelectedData :type SS%20Augment%20Data%20Object%20Reference))
  (bind _returnvalue (Game|GetPlayerCharacter 0))
  (bind _returnvalue_2 (Game|GetPlayerController 0))
  (bind _value (Variables|/Script/SuperSimple.SSAugmentData|GetValue SelectedData))
  (switch Utilities|FlowControl|Switch|SwitchonEAugmentType (Variables|/Script/SuperSimple.SSAugmentData|GetAugmentType SelectedData)
    (:SpeedUp
      (bind _asbp_player (Utilities|Casting|CastToBP_Player _returnvalue))
      (Variables|/Script/Engine.CharacterMovementComponent|SetMaxWalkSpeed (Variables|/Script/Engine.Character|GetCharacterMovement _asbp_player) (+ (Variables|/Script/Engine.CharacterMovementComponent|GetMaxWalkSpeed (Variables|/Script/Engine.Character|GetCharacterMovement _asbp_player)) _value)))
    (:MaxHealthUp
      (bind _asbp_player_2 (Utilities|Casting|CastToBP_Player _returnvalue))
      (Variables|/Script/SuperSimple.SSCharacter|SetMaxHealth _asbp_player_2 (Math|Float|Truncate (+ (Variables|/Script/SuperSimple.SSCharacter|GetMaxHealth _asbp_player_2) _value))))
    (:Weapon
      (bind _asbp_player_3 (Utilities|Casting|CastToBP_Player _returnvalue))
      (Class|SSCharacter|SwapWeapon _asbp_player_3 (Variables|/Script/SuperSimple.SSAugmentData|GetWeaponReward SelectedData)))
    (:ReloadSpeed
      (bind _asbp_player_4 (Utilities|Casting|CastToBP_Player _returnvalue))
      (Variables|/Script/SuperSimple.SSCharacter|SetReloadSpeedMultiplier _asbp_player_4 (* _value (Variables|/Script/SuperSimple.SSCharacter|GetReloadSpeedMultiplier _asbp_player_4))))
    (:FireRate
      (bind _asbp_player_5 (Utilities|Casting|CastToBP_Player _returnvalue))
      (Variables|/Script/SuperSimple.SSCharacter|SetFireRateMultiplier _asbp_player_5 (* _value (Variables|/Script/SuperSimple.SSCharacter|GetFireRateMultiplier _asbp_player_5))))
    (:ProjectileSpeed
      (bind _asbp_player_6 (Utilities|Casting|CastToBP_Player _returnvalue))
      (Variables|/Script/SuperSimple.SSCharacter|SetProjectileSpeedMultiplier _asbp_player_6 (* _value (Variables|/Script/SuperSimple.SSCharacter|GetProjectileSpeedMultiplier _asbp_player_6))))
    (:Ricochet
      (bind _asbp_player_7 (Utilities|Casting|CastToBP_Player _returnvalue))
      (bind _result (Math|Integer|IncrementInt (Variables|/Script/SuperSimple.SSCharacter|GetBonusRicochetCount _asbp_player_7))
        (:%20%20
          (Variables|/Script/SuperSimple.SSCharacter|SetBonusRicochetCount _asbp_player_7 _result))))
    (:Pierce
      (bind _asbp_player_8 (Utilities|Casting|CastToBP_Player _returnvalue))
      (bind _result_2 (Math|Integer|IncrementInt (Variables|/Script/SuperSimple.SSCharacter|GetBonusPierceCount _asbp_player_8))
        (:%20%20
          (Variables|/Script/SuperSimple.SSCharacter|SetBonusPierceCount _asbp_player_8 _result_2)))))
  (Widget|RemovefromParent (stale Custom|LevelUpSequence _output_get))
  (Game|SetGamePaused false)
  (Input|SetInputModeGameOnly _returnvalue_2 false)
  (Variables|/Script/Engine.PlayerController|SetbShowMouseCursor _returnvalue_2 false))

(event EventBeginPlay
  (bind _returnvalue (Game|GetPlayerController 0))
  (bind _bgm_list (Variables|Default|GetBGM_List))
  (bind _returnvalue_2 (UserInterface|CreateWidget "/Game/Blueprints/WBP_HUD.WBP_HUD_C" _returnvalue))
  (Variables|Default|SetMainHUD _returnvalue_2)
  (UserInterface|Viewport|AddtoViewport _returnvalue_2 0)
  (Input|SetInputModeGameOnly _returnvalue false)
  (Variables|/Script/Engine.PlayerController|SetbShowMouseCursor _returnvalue false)
  (bind _returnvalue_3 (Audio|SpawnSound2D (Utilities|Array|Get(acopy) _bgm_list (Math|Random|RandomIntegerinRange 0 (Utilities|Array|LastIndex _bgm_list))) 1.0 1.0 0.0 0))
  (Variables|Components|SetCurrentMusicComp _returnvalue_3)
  (EventDispatchers|AssignOnScoreChanged (delegate Custom|OnScoreChanged_Event)))

(event EventOnGameOver
  (bind _returnvalue (Game|GetPlayerController 0))
  (Game|SetGamePaused true)
  (Variables|/Script/Engine.PlayerController|SetbShowMouseCursor _returnvalue true)
  (Input|SetInputModeUIOnly _returnvalue 0 "DoNotLock" false)
  (bind _returnvalue_2 (UserInterface|CreateWidget "/Game/Blueprints/WBP_GameOver.WBP_GameOver_C" _returnvalue (Variables|Default|GetTotalScore) (Variables|Default|GetCurrentWave)))
  (UserInterface|Viewport|AddtoViewport _returnvalue_2 0))

(event EventOnLevelUp
  (CallFunction|LevelUpSequence))

(event EventTick
  (params (DeltaSeconds :type Float%20%28single-precision%29))
  (bind _currentmusiccomp (Variables|Components|GetCurrentMusicComp))
  (Utilities|IsValid _currentmusiccomp
    (:Is%20Valid
      (Audio|Components|Audio|SetPitchMultiplier _currentmusiccomp (Math|Interpolation|FInterpTo (Variables|Default|GetCurrentPitch) (Math|Float|SelectFloat 0.6 1.0 (<= (Variables|/Script/SuperSimple.SSCharacter|GetCurrentHealth (.AsBP%20Player (Utilities|Casting|CastToBP_Player (Game|GetPlayerCharacter 0)))) 1)) DeltaSeconds 1.0))
      (Variables|Default|SetCurrentPitch (Math|Interpolation|FInterpTo (Variables|Default|GetCurrentPitch) (Math|Float|SelectFloat 0.6 1.0 (<= (Variables|/Script/SuperSimple.SSCharacter|GetCurrentHealth (.AsBP%20Player (Utilities|Casting|CastToBP_Player (Game|GetPlayerCharacter 0)))) 1)) DeltaSeconds 1.0)))))

(fn ConstructionScript)