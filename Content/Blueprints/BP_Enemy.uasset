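; Enemy character that takes one point of damage per hit and reports its death to BP_GameMode.
; On spawn, a weighted random pick from VariantList sets the mesh overlay material and XP reward.
; At zero health it ragdolls with an impulse along its velocity, awarding variant XP only for player bullet kills, then destroys itself after a delay.
; Tick removes it without XP if it strays too far from world origin.
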(event Custom|ApplyRandomVariant
  (bind _variantlist (Variables|Default|GetVariantList))
  (for _array_element _variantlist
    (Variables|Default|SetTotalWeight (+ (.spawnrate _array_element) (Variables|Default|GetTotalWeight))))
  (Variables|Default|SetRandomPick (Math|Random|RandomFloatinRange 0.0 (Variables|Default|GetTotalWeight)))
  (bind _array_element_2 (Utilities|Array|ForEachLoopwithBreak _variantlist :!label _label)
    (:LoopBody
      (Variables|Default|SetCustomSum (+ (.spawnrate _array_element_2) (Variables|Default|GetCustomSum)))
      (if (<= (Variables|Default|GetRandomPick) (Variables|Default|GetCustomSum))
        (Rendering|Material|SetOverlayMaterial (Variables|Character|GetMesh) (.overlaymaterial _array_element_2) :!class /Script/Engine.MeshComponent)
        (Variables|Default|SetCurrentVariantXP (.bonusxp _array_element_2))
        (goto _label Break)))))

(event EventBeginPlay
  (Variables|Default|SetGunMeshComp (Variables|Default|GetGun))
  (CallFunction|ApplyRandomVariant))

(event EventTakeDamage
  (params (DamageAmount :type Float%20%28single-precision%29) (DamageCauser :type Actor%20Object%20Reference))
  (bind _mesh (Variables|Character|GetMesh))
  (bind _output_get (Variables|Default|SetHealth (- (Variables|Default|GetHealth) 1)))
  (if (== _output_get 0)
    (Class|SSEnemy|SetEnemyDead)
    (bind _asbp_game_mode (Utilities|Casting|CastToBP_GameMode (Game|GetGameMode)))
    (Utilities|Casting|CastToBP_PlayerBullet DamageCauser
      (:then
        (Class|SSGameMode|OnEnemyKilled _asbp_game_mode (Variables|Default|GetCurrentVariantXP) (Game|GetInstigator DamageCauser)))
      (:CastFailed
        (Class|SSGameMode|OnEnemyKilled _asbp_game_mode)))
    (Collision|SetCollisionProfileName _mesh "Ragdoll" true :!class /Script/Engine.PrimitiveComponent)
    (Physics|SetSimulatePhysics _mesh true)
    (Collision|SetCollisionResponsetoChannel (Variables|Character|GetMesh) "ECC_GameTraceChannel1" "ECR_Ignore")
    (Collision|SetCollisionEnabled (Variables|Default|GetCapsuleComponent) "NoCollision")
    (Physics|AddImpulseatLocation _mesh (* (Math|Vector|Normalize (Transformation|GetVelocity)) "100000.000000,100000.000000,100000.000000") (Transformation|GetActorLocation) "None")
    (Utilities|FlowControl|Delay 3.0)
    (Actor|DestroyActor)))

(event EventTick
  (params (DeltaSeconds :type Float%20%28single-precision%29))
  (if (> (Math|Vector|VectorLength (Transformation|GetActorLocation)) 5e+03)
    (Variables|Default|SetHealth 0)
    (bind _asbp_game_mode (Utilities|Casting|CastToBP_GameMode (Game|GetGameMode)))
    (Class|SSGameMode|OnEnemyKilled _asbp_game_mode)
    (Actor|DestroyActor)))

(fn ConstructionScript)